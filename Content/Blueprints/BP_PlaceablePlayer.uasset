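; BP_PlaceablePlayer is a player character stand-in whose Mesh plays a looping idle animation from BeginPlay.
; It plays animation assets directly on the Mesh through PlayAnimation.
; An unconnected branch would choose running, forward flip or idle from walk and jump flags, then clear AnimationPlay, but it never runs.
; Tick and the construction script are empty.
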(event EventBeginPlay
  (Components|Animation|PlayAnimation (Variables|Character|GetMesh) "/Game/Characters/Mixamo/Anim/Idle_mixamo_com.Idle_mixamo_com" true))

(event Collision|EventActorBeginOverlap
  (params (OtherActor :type Actor%20Object%20Reference)))

(event EventTick
  (params (DeltaSeconds :type Float%20%28single-precision%29)))

(fn ConstructionScript)