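; BP_GunPickup is an AR pistol pickup that becomes the player's touch-fired weapon once the game state marks it collected.
; Tick polls that flag, then once attaches the gun to the pawn's CamManager, aligns the mesh to GunChild and swaps in the collected material.
; Touch plays fire animation and sound, spends game-state ammo and calls the pawn's Shoot, adding a zombie-hit sound on hits.
; An empty magazine triggers a delayed reload from reserves.
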(event EventBeginPlay
  (bind _ascustom_game_state (Utilities|Casting|CastToCustomGameState (Game|GetGameState)))
  (Variables|Default|SetGS _ascustom_game_state)
  (Input|EnableInput (Game|GetPlayerController 0))
  (Transformation|SetActorRotation "90.000000, 0, 0")
  (bind _ascustom_arpawn (Utilities|Casting|CastToCustomARPawn (Game|Player|GetPlayerPawn 0)))
  (Variables|Default|SetAs%20Custom%20ARPawn _ascustom_arpawn))

(event Collision|EventActorBeginOverlap
  (params (OtherActor :type Actor%20Object%20Reference)))

(event EventTick
  (params (DeltaSeconds :type Float%20%28single-precision%29))
  (bind _skeletalmesh (Variables|Default|GetSkeletalMesh))
  (Utilities|FlowControl|Sequence
    (:then_0
      (bind _returnvalue (Class|CustomGameState|GetIsIsGunCollected (Variables|Default|GetGS)))
      (if _returnvalue
        (if (not (Variables|Default|GetIsGunPicked_0))
          (bind _asbp_custom_arpawn (Utilities|Casting|CastToBP_CustomARPawn (Pawn|GetControlledPawn (Game|GetPlayerController 0))))
          (Transformation|AttachActorToActor (Variables|/Script/UE5_AR.CustomARPawn|GetcamManager _asbp_custom_arpawn) "None" "KeepRelative" "KeepWorld" "KeepRelative" true)
          (Transformation|SetRelativeLocation _skeletalmesh (Variables|/Script/Engine.SceneComponent|GetRelativeLocation (Variables|/Game/Blueprints/BP_CustomARPawn.BP_CustomARPawn_C|GetGunChild _asbp_custom_arpawn)) false false)
          (Transformation|SetRelativeRotation _skeletalmesh (Variables|/Script/Engine.SceneComponent|GetRelativeRotation (Variables|/Game/Blueprints/BP_CustomARPawn.BP_CustomARPawn_C|GetGunChild _asbp_custom_arpawn)) false false)
          (Variables|Default|SetIsGunPicked_0 true))))
    (:then_1
      (if (not (Variables|Default|GetFlipMaterial))
        (if (Variables|Default|GetIsGunPicked_0)
          (Rendering|Material|SetMaterial (Variables|Default|GetSkeletalMesh) 0 "/Game/MilitaryWeapSilver/Weapons/Textures/Pistols_A_MatCollected.Pistols_A_MatCollected")
          (Variables|Default|SetFlipMaterial true))))))

(event Input|TouchEvents|Touch1
  (params (Key :type Key%20Structure :default "None"))
  (bind _gs (Variables|Default|GetGS))
  (bind _gs_2 (Variables|Default|GetGS))
  (bind _as_custom_arpawn (Variables|Default|GetAs%20Custom%20ARPawn))
  (:Pressed
    (bind _returnvalue (Class|CustomGameState|GetIsIsGunCollected (Variables|Default|GetGS)))
    (if _returnvalue
      (if (not (Audio|Components|Audio|IsPlaying (Variables|Default|GetSkeletalMesh)))
        (bind _returnvalue_2 (Class|CustomGameState|GetAmmo (Variables|Default|GetGS)))
        (if (> _returnvalue_2 0)
          (Components|Animation|PlayAnimation (Variables|Default|GetSkeletalMesh) "/Game/MilitaryWeapSilver/Weapons/Animations/Fire_Pistol_W.Fire_Pistol_W" false)
          (Audio|PlaySound2D "/Game/MilitaryWeapSilver/Sound/Pistol/Wavs/PistolA_Fire01.PistolA_Fire01" 1.0 1.0 0.0 0 0)
          (bind _returnvalue_3 (Class|CustomGameState|GetAmmo _gs_2))
          (Class|CustomGameState|SetAmmo _gs_2 (- _returnvalue_3 1))
          (Class|CustomARPawn|Shoot _as_custom_arpawn)
          (if (Variables|/Script/UE5_AR.CustomARPawn|GetZombieHit _as_custom_arpawn)
            (Audio|PlaySound2D "/Game/Sound/Y2Mate_is_-_Minecraft_Zombie_Hit_-_Sound_Effect-DOTj_aJLHvw-128k-1656945423623.Y2Mate_is_-_Minecraft_Zombie_Hit_-_Sound_Effect-DOTj_aJLHvw-128k-1656945423623" 1.0 1.0 0.0 0 0)
            (Variables|/Script/UE5_AR.CustomARPawn|SetZombieHit _as_custom_arpawn false))
          (else
            (bind _returnvalue_4 (Class|CustomGameState|GetAmmoReload (Variables|Default|GetGS)))
            (if (> _returnvalue_4 0)
              (Components|Animation|PlayAnimation (Variables|Default|GetSkeletalMesh) "/Game/MilitaryWeapSilver/Weapons/Animations/Reload_Pistol_W.Reload_Pistol_W" false)
              (Utilities|FlowControl|Delay 1.0)
              (Class|CustomGameState|SetAmmo _gs 10)
              (bind _returnvalue_5 (Class|CustomGameState|GetAmmoReload _gs))
              (Class|CustomGameState|SetAmmoReload _gs (- _returnvalue_5 1)))))))))

(fn ConstructionScript)