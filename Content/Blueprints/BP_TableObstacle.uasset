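; BP_TableObstacle is an AR table obstacle that counts how often the player walks into it.
; It caches the custom AR pawn and game state at BeginPlay, then checks each Tick the horizontal distance to the pawn's camera location.
; Coming within a fixed radius increments the game state's table collision count, with two flags limiting it to once per approach.
; Overlap events are empty, so detection is purely distance-based.
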(event OnComponentBeginOverlap(BoxComponent)
  (params (OverlappedComponent :type Primitive%20Component%20Object%20Reference) (OtherActor :type Actor%20Object%20Reference) (OtherComp :type Primitive%20Component%20Object%20Reference) (OtherBodyIndex :type Integer) (bFromSweep :type Boolean) (SweepResult :type Hit%20Result%20Structure%20%28by%20ref%29)))

(event EventBeginPlay
  (bind _ascustom_arpawn (Utilities|Casting|CastToCustomARPawn (Game|Player|GetPlayerPawn 0)))
  (Variables|Default|SetCustom%20ARPawn _ascustom_arpawn)
  (bind _ascustom_game_state (Utilities|Casting|CastToCustomGameState (Game|GetGameState)))
  (Variables|Default|SetCustomGameState _ascustom_game_state))

(event Collision|EventActorBeginOverlap
  (params (OtherActor :type Actor%20Object%20Reference)))

(event EventTick
  (params (DeltaSeconds :type Float%20%28single-precision%29))
  (bind _returnvalue (Transformation|GetActorLocation))
  (bind _custom_arpawn (Variables|Default|GetCustom%20ARPawn))
  (bind _customgamestate (Variables|Default|GetCustomGameState))
  (bind _camlocation (Variables|/Script/UE5_AR.CustomARPawn|GetcamLocation _custom_arpawn))
  (Utilities|FlowControl|Sequence
    (:then_0
      (if (<= (Math|Vector2D|Vector2DLength (- (Math|Vector2D|MakeVector2D (.x _returnvalue) (.y _returnvalue)) (Math|Vector2D|MakeVector2D (.x _camlocation) (.y _camlocation)))) 75.0)
        (if (not (Variables|Default|GetIsColliding))
          (if (Variables|Default|GetShouldCollide)
            (bind _returnvalue_2 (Class|CustomGameState|GetTableCollisions _customgamestate))
            (Class|CustomGameState|SetTableCollisions _customgamestate (+ _returnvalue_2 1))
            (Variables|Default|SetIsColliding true)
            (Variables|Default|SetShouldCollide false)))
        (else
          (Variables|Default|SetShouldCollide true)
          (Variables|Default|SetIsColliding false))))))

(fn ConstructionScript)