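; Spawned zombie enemy for an AR game that plays a stand-up animation, then attacks the player at close range.
; Tick drives an EnemyStatus state machine from camera distance, switching between attack and running animations.
; Attacks subtract health from CustomGameState on a cooldown, with timed force-feedback rumble while attacking.
; Health below its starting value triggers a damage widget animation with fixed text, and a component rotates to face the camera.
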(event OnComponentBeginOverlap(CapsuleComponent)
  (params (OverlappedComponent :type Primitive%20Component%20Object%20Reference) (OtherActor :type Actor%20Object%20Reference) (OtherComp :type Primitive%20Component%20Object%20Reference) (OtherBodyIndex :type Integer) (bFromSweep :type Boolean) (SweepResult :type Hit%20Result%20Structure%20%28by%20ref%29)))

(event OnComponentEndOverlap(CapsuleComponent)
  (params (OverlappedComponent :type Primitive%20Component%20Object%20Reference) (OtherActor :type Actor%20Object%20Reference) (OtherComp :type Primitive%20Component%20Object%20Reference) (OtherBodyIndex :type Integer)))

(event EventBeginPlay
  (Variables|Default|SetEnemyStatus "Spawning")
  (Components|Animation|PlayAnimation (Variables|Character|GetMesh) "/Game/Characters/Mixamo/Anim/Zombie_Stand_Up.Zombie_Stand_Up" false)
  (bind _ascustom_game_state (Utilities|Casting|CastToCustomGameState (Game|GetGameState)))
  (Variables|Default|SetGS _ascustom_game_state)
  (bind _ascustom_game_mode (Utilities|Casting|CastToCustomGameMode (Game|GetGameMode)))
  (Variables|Default|SetGM _ascustom_game_mode)
  (bind _ascustom_arpawn (Utilities|Casting|CastToCustomARPawn (Game|Player|GetPlayerPawn 0)))
  (Variables|Default|SetCustomARPawn _ascustom_arpawn)
  (Variables|Default|SetTmpHealth (Variables|Default|GetHealth))
  (bind _returnvalue (UserInterface|CreateWidget "/Game/UI/GameUI/EnemyDamageUI.EnemyDamageUI_C"))
  (Variables|Default|SetNewVar_0 _returnvalue))

(event EventTick
  (params (DeltaSeconds :type Float%20%28single-precision%29))
  (bind _mesh (Variables|Character|GetMesh))
  (bind _gs (Variables|Default|GetGS))
  (Utilities|FlowControl|Sequence
    (:then_0
      (if (not (Variables|Default|GetInCooldown))
        (if (== (Math|Conversions|ToInteger(Byte) (Variables|Default|GetEnemyStatus)) 4)
          (Components|Animation|PlayAnimation (Variables|Character|GetMesh) "/Game/Characters/Mixamo/Anim/Zombie_Attack_mixamo_com.Zombie_Attack_mixamo_com" false)
          (bind _returnvalue (Class|CustomGameState|GetHealth _gs))
          (Class|CustomGameState|SetHealth _gs (- _returnvalue 20))
          (Variables|Default|SetInCooldown true))))
    (:then_1
      (if (Variables|Default|GetInCooldown)
        (Variables|Default|SetAttackCooldown (+ (Variables|Default|GetAttackCooldown) DeltaSeconds))
        (if (> (Variables|Default|GetAttackCooldown) 2.0)
          (Variables|Default|SetInCooldown false)
          (Variables|Default|SetAttackCooldown 0.0))))
    (:then_2
      (if (== (Math|Conversions|ToInteger(Byte) (Variables|Default|GetEnemyStatus)) 5)
        (if (not (Audio|Components|Audio|IsPlaying _mesh))
          (Components|Animation|SetAnimationMode _mesh "AnimationBlueprint")
          (Variables|Default|SetEnemyStatus "Idle"))))
    (:then_3
      (if (< (Math|Vector|VectorLength (- (Variables|/Script/UE5_AR.CustomARPawn|GetcamLocation (Variables|Default|GetCustomARPawn)) (Transformation|GetActorLocation))) 1e+02)
        (if (not (Variables|Default|GetInCooldown))
          (Variables|Default|SetEnemyStatus "Attacking"))
        (elif (== (Math|Conversions|ToInteger(Byte) (Variables|Default|GetEnemyStatus)) 4)
          (Variables|Default|SetEnemyStatus "Charging")
          (Components|Animation|PlayAnimation (Variables|Character|GetMesh) "/Game/Characters/Mixamo/Anim/Zombie_Running.Zombie_Running" true))))
    (:then_4
      (if (== (Math|Conversions|ToInteger(Byte) (Variables|Default|GetEnemyStatus)) 4)
        (if (> (Variables|Default|GetVibrate) 0.5)
          (Utilities|FlowControl|Sequence
            (:then_0
              (goto _label Stop))
            (:then_1
              (Variables|Default|SetVibrate 0.0)))
          (else
            (Variables|Default|SetVibrate (+ (Variables|Default|GetVibrate) DeltaSeconds))
            (Game|Feedback|PlayDynamicForceFeedback (Game|GetPlayerController 0) 0.8 -1.0 true true true true :!label _label)
            (Variables|Default|SetVibrate 0.0)))
        (else
          (goto _label Stop))))
    (:then_5
      (if (> (Variables|Default|GetTmpHealth) (Variables|Default|GetHealth))
        (bind _asenemy_damage_ui (Utilities|Casting|CastToEnemyDamageUI (UserInterface|GetWidget)))
        (Default|PlayDMGAnimation _asenemy_damage_ui "-50")))
    (:then_6
      (Transformation|SetWorldRotation (Math|Rotator|FindLookatRotation (Transformation|GetWorldLocation) (Camera|GetCameraLocation (Game|GetPlayerCameraManager 0))) false false))))

(fn ConstructionScript)