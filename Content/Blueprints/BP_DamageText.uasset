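; Floating damage number actor that shows the random damage value of the player's CustomARPawn in an AR game.
; On BeginPlay it sets the text from that pawn's RandomDamage and picks a random, upward-biased drift vector.
; Each Tick it billboards toward the camera, moves along that vector, and destroys itself after a short lifetime.
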(event EventBeginPlay
  (bind _ascustom_arpawn (Utilities|Casting|CastToCustomARPawn (Game|Player|GetPlayerPawn 0)))
  (Variables|Default|SetPawnRef (Game|GetPlayerCameraManager 0))
  ;[1 1 1] Set text to damage randomly generated.
  (Rendering|Components|TextRender|SetText (Variables|Default|GetDmgTxt) (Utilities|Text|MakeLiteralText (Utilities|Text|ToText(Integer) (Variables|/Script/UE5_AR.CustomARPawn|GetRandomDamage _ascustom_arpawn))))
  (Transformation|SetActorRotation "0, 0, 0")
  ;[1 1 1] Move towards a random direction, with positive z.
  (Variables|Default|SetLifeTime 2.0)
  (Variables|Default|SetMovementVector (Math|Vector|MakeVector (Math|Random|RandomFloatinRange 0.0 5e+01) (Math|Random|RandomFloatinRange -1.5e+02 1.5e+02) (Math|Random|RandomFloatinRange 0.0 1.5e+02))))

(event Collision|EventActorBeginOverlap
  (params (OtherActor :type Actor%20Object%20Reference)))

(event EventTick
  (params (DeltaSeconds :type Float%20%28single-precision%29))
  ;[1 1 1] Rotate text towards player.
  (Transformation|SetActorRotation (Math|Conversions|RotationFromXVector (Math|Vector|Normalize (- (Camera|GetCameraLocation (Variables|Default|GetPawnRef)) (Transformation|GetActorLocation)))))
  ;[1 1 1] Update lifetime and move towards movement vector
  (Variables|Default|SetLifeTime (- (Variables|Default|GetLifeTime) DeltaSeconds))
  (Transformation|SetActorLocation (+ (Transformation|GetActorLocation) (* (Variables|Default|GetMovementVector) DeltaSeconds)) false false)
  ;[1 1 1] Destroy actor after lifetime reaches zero.
  (if (<= (Variables|Default|GetLifeTime) 0.0)
    (Actor|DestroyActor)))

(fn ConstructionScript)